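; Butterfly spawner actor that compares two swarms driven by separate Sigma, Rho and Beta setups, the parameters of a Lorenz attractor.
; BeginPlay spawns each swarm as offset butterfly components with attached particle systems and shows its parameters in a compare widget.
; Every Tick, UpdatePosition computes each butterfly's next relative location from its current one and its swarm's setup.
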(event `self.ReceiveBeginPlay`
  (`|ExecutionSequence`
    (:`then_0`
      (bind _meshbutterarray (`self.SetupButterfly` (`|GetArrayItem` (`self.ButterflySetupArray`)) (`self.WidgetButterfly1`)))
      (set `self.MeshArray_1` _meshbutterarray))
    (:`then_1`
      (bind _meshbutterarray_2 (`self.SetupButterfly` (`|GetArrayItem` (`self.ButterflySetupArray`) 1) (`self.WidgetButterfly2`)))
      (set `self.MeshArray_2` _meshbutterarray_2))))

(event `self.ReceiveTick`
  (params (DeltaSeconds :type "Float (single-precision)"))
  (`self.UpafeteButteflyLocation` (`self.MeshArray_1`) (`|GetArrayItem` (`self.ButterflySetupArray`)))
  (`self.UpafeteButteflyLocation` (`self.MeshArray_2`) (`|GetArrayItem` (`self.ButterflySetupArray`) 1)))

(fn `SetupButterfly`
  (params (ButerflySetup :type "ButterflySetup Structure") (Widget :type "WidgetComponent Object Reference"))
  (returns (MeshButterArray :type "Array of StaticMeshComponent Object Reference"))
  (locals (NewLocalVar_0 :type "Array of StaticMeshComponent Object Reference"))
  (bind (_sigma _rho _beta) (break `ButterflySetup` ButerflySetup))
  (`|ExecutionSequence`
    (:`then_0`
      (for _index (range (+ (`self.numberOfButterfly`) 1))
        (`|ExecutionSequence`
          (:`then_0`
            (bind _returnvalue (`|AddComponentByClass` "/Script/Engine.ParticleSystemComponent" false (`KismetMathLibrary.MakeTransform` (0.0 0.0 0.0) (struct) (`KismetMathLibrary.Conv_DoubleToVector` (`self.ButterflyScale`)))))
            (`ParticleSystemComponent.SetTemplate` _returnvalue "/Game/BluePrints/Butterfly/ParticleSystemButterfly.ParticleSystemButterfly"))
          (:`then_1`
            (bind _returnvalue_2 (`|AddComponentByClass` "/Game/BluePrints/Butterfly/BP_ButterflyComp.BP_ButterflyComp_C" false (`KismetMathLibrary.MakeTransform` (`KismetMathLibrary.MakeVector` (* _index 15.0) 3.0 6.0) (struct) (`KismetMathLibrary.Conv_DoubleToVector` (`self.ButterflyScale`)))))
            (`SceneComponent.K2_AttachToComponent` _returnvalue _returnvalue_2 "None" "SnapToTarget" "SnapToTarget" "KeepWorld" true)
            (`KismetArrayLibrary.Array_Add` (`local.NewLocalVar_0`) _returnvalue_2)))))
    (:`then_1`
      (bind _aswbp_butterfly_compare (cast `/Game/BluePrints/Butterfly/WBP_ButterflyCompare` (`WidgetComponent.GetUserWidgetObject` Widget)))
      (`/Game/BluePrints/Butterfly/WBP_ButterflyCompare.SetButterflyInfo` :`self` _aswbp_butterfly_compare :`Sigma` _sigma :`Rho` _rho :`Beta` _beta))
    (:`then_2`
      (return (`local.NewLocalVar_0`)))))

(fn `UpafeteButteflyLocation`
  (params (Array :type "Array of StaticMeshComponent Object Reference") (ButterflySetup :type "ButterflySetup Structure"))
  (for _array_element Array
    (bind _returnvalue (`self.UpdatePosition` ButterflySetup (`SceneComponent.RelativeLocation` _array_element)))
    (`SceneComponent.K2_SetRelativeLocation` _array_element _returnvalue false false)))

(fn `UserConstructionScript`)