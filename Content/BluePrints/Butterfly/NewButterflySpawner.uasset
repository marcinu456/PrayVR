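; Butterfly spawner Blueprint that creates a small group of animated-position butterflies at runtime.
; BeginPlay adds four scaled BP_ButterflyComp components spaced along local X, each with an attached butterfly particle system, and stores them in MeshArray.
; Tick passes each component's relative location through UpdatePosition, whose logic is not defined in this graph, and applies the result without sweeping.
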(event `self.ReceiveBeginPlay`
  (`|ExecutionSequence`
    (:`then_0`
      (for _index (range 4)
        (`|ExecutionSequence`
          (:`then_0`
            (bind _returnvalue (`|AddComponentByClass` "/Script/Engine.ParticleSystemComponent" false (`KismetMathLibrary.MakeTransform` (0.0 0.0 0.0))))
            (`ParticleSystemComponent.SetTemplate` _returnvalue "/Game/BluePrints/Butterfly/ParticleSystemButterfly.ParticleSystemButterfly"))
          (:`then_1`
            (bind _returnvalue_2 (`|AddComponentByClass` "/Game/BluePrints/Butterfly/BP_ButterflyComp.BP_ButterflyComp_C" false (`KismetMathLibrary.MakeTransform` (`KismetMathLibrary.MakeVector` (* _index 15.0) 3.0 6.0) (struct) (`KismetMathLibrary.Conv_DoubleToVector` (`self.ButterflyScale`)))))
            (`SceneComponent.K2_AttachToComponent` _returnvalue _returnvalue_2 "None" "SnapToTarget" "SnapToTarget" "SnapToTarget" true)
            (`KismetArrayLibrary.Array_Add` (`self.MeshArray`) _returnvalue_2)))))))

(event `self.ReceiveTick`
  (params (DeltaSeconds :type "Float (single-precision)"))
  (for _array_element (`self.MeshArray`)
    (bind _returnvalue (`self.UpdatePosition` (`SceneComponent.RelativeLocation` _array_element)))
    (`SceneComponent.K2_SetRelativeLocation` _array_element _returnvalue false false)))

(fn `UserConstructionScript`)