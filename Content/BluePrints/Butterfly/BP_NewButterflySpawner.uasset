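; Butterfly spawner actor that creates a set of particle-trailed butterflies and moves them every frame.
; BeginPlay spawns NumberOfButterfly-driven BP_ButterflyComp components at staggered X offsets, attaches a particle system to each and stores them in MeshArray.
; It also passes the first setup entry's Lorenz-attractor parameters (Sigma, Rho, Beta) to the WBP_Butterfly widget.
; Tick feeds each component's relative location through UpdatePosition and applies the result.
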(event `self.ReceiveBeginPlay`
  (bind (_sigma _rho _beta) (break `ButterflySetup` (`|GetArrayItem` (`self.ButterflySetupArray`))))
  (`|ExecutionSequence`
    (:`then_0`
      (for _index (range (+ (`self.numberOfButterfly`) 1))
        (`|ExecutionSequence`
          (:`then_0`
            (bind _returnvalue (`|AddComponentByClass` "/Script/Engine.ParticleSystemComponent" false (`KismetMathLibrary.MakeTransform` (0.0 0.0 0.0) (struct) (`KismetMathLibrary.Conv_DoubleToVector` (`self.ButterflyScale`)))))
            (`ParticleSystemComponent.SetTemplate` _returnvalue "/Game/BluePrints/Butterfly/ParticleSystemButterfly.ParticleSystemButterfly"))
          (:`then_1`
            (bind _returnvalue_2 (`|AddComponentByClass` "/Game/BluePrints/Butterfly/BP_ButterflyComp.BP_ButterflyComp_C" false (`KismetMathLibrary.MakeTransform` (`KismetMathLibrary.MakeVector` (* _index 15.0) 3.0 6.0) (struct) (`KismetMathLibrary.Conv_DoubleToVector` (`self.ButterflyScale`)))))
            (`SceneComponent.K2_AttachToComponent` _returnvalue _returnvalue_2 "None" "SnapToTarget" "SnapToTarget" "KeepWorld" true)
            (`KismetArrayLibrary.Array_Add` (`self.MeshArray`) _returnvalue_2)))))
    (:`then_1`
      (bind _aswbp_butterfly (cast `/Game/BluePrints/Butterfly/WBP_Butterfly` (`WidgetComponent.GetUserWidgetObject` (`self.Widget`))))
      (`/Game/BluePrints/Butterfly/WBP_Butterfly.SetButterflyInfo` _aswbp_butterfly _sigma _rho _beta))))

(event `self.ReceiveTick`
  (params (DeltaSeconds :type "Float (single-precision)"))
  (for _array_element (`self.MeshArray`)
    (bind _returnvalue (`self.UpdatePosition` (struct) (`SceneComponent.RelativeLocation` _array_element)))
    (`SceneComponent.K2_SetRelativeLocation` _array_element _returnvalue false false)))

(fn `UserConstructionScript`)