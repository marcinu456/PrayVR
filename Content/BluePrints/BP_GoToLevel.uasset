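; BP_GoToLevel is a level portal actor that loads another level when the player walks into it.
; On BeginPlay it shows its LevelName on a TextRender component as a label.
; When an overlapping actor is the first player character, it prints a message and opens that level by name.
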(event `self.ReceiveBeginPlay`
  (`TextRenderComponent.K2_SetText` (`self.TextRender`) (`KismetTextLibrary.Conv_NameToText` (`self.LevelName`))))

(event `self.ReceiveActorBeginOverlap`
  (params (OtherActor :type "Actor Object Reference"))
  (bind _levelname (`self.LevelName`))
  (if (== OtherActor (`GameplayStatics.GetPlayerCharacter` 0))
    (`KismetSystemLibrary.PrintString` (`KismetStringLibrary.Concat_StrStr` "Go to level " (`KismetStringLibrary.Conv_NameToString` _levelname)) true true (struct :`G` 0.66 :`B` 1.0 :`A` 1.0) 12.0)
    (`GameplayStatics.OpenLevel` _levelname)))

(fn `UserConstructionScript`)